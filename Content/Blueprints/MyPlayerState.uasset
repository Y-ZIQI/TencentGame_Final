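; MyPlayerState is a player state Blueprint that holds a player's name, score and death count.
; Its construction script reads the base name from MyGameInstance and appends a random number below 1000 to form PlayerName.
; IncrementScore and IncrementDeath each add one to their counter, and the event graph has no active logic.
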(fn `IncrementDeath`
  (set `self.PlayerDeath` (+ (`self.PlayerDeath`) 1)))

(fn `IncrementScore`
  (set `self.PlayerScore` (+ (`self.PlayerScore`) 1)))

(fn `UserConstructionScript`
  (bind _asmy_game_instance (cast `/Game/Blueprints/MyGameInstance` (`GameplayStatics.GetGameInstance`)))
  (set `self.PlayerName` (`KismetStringLibrary.Concat_StrStr` (`/Game/Blueprints/MyGameInstance.PlayerName` _asmy_game_instance) (`KismetStringLibrary.Conv_IntToString` (`KismetMathLibrary.RandomInteger` 1000)))))