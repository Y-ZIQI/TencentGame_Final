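; Game instance that drives front-end menu flow and online session hosting, searching and joining.
; A state machine removes the previous screen's widget or destroys the session on leaving gameplay, then lazily creates and shows the next widget.
; Advanced Sessions nodes store room name and password as extra settings, checked client-side before joining.
; A parallel set of "WithMySession" events uses a custom MySessionSubsystem, including the destroy-on-exit call.
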(event `ShowMainMenu`
  (bind _returnvalue (`GameplayStatics.GetPlayerController` 0))
  (bind _mainmenu (`self.MainMenu`))
  (`self.IsCurrentState` "NewEnumerator3"
    (:`True`
      (`GameplayStatics.OpenLevel` "MainMenuMap")
      (`KismetSystemLibrary.Delay` 0.2))
    (:`False`
      _))
  (`self.TransitionToState` "NewEnumerator1"
    (:`NewState`
      (`/Engine/EditorBlueprintResources/StandardMacros.IsValid` (`self.MainMenu`)
        (:`Is Valid`
          _)
        (:`Is Not Valid`
          (bind _returnvalue_2 (`|CreateWidget` "/Game/Blueprints/Widgets/MainMenu/MainMenu.MainMenu_C" _returnvalue))
          (set `self.MainMenu` _returnvalue_2)))
      (`WidgetBlueprintLibrary.SetInputMode_UIOnlyEx` _returnvalue _mainmenu)
      (`UserWidget.AddToViewport` _mainmenu 0))))

(event `JoinFromServerListEvent(With MySession)`
  (params (MySession :type "MySession Structure"))
  ;[1 1 1] Action with MySession
  (`MySessionSubsystem.JoinSession` (`self.MySessionSubsystem`) (`.SessionName` (break `MySession` MySession))))

(event `HostGame(With MySession)`
  ;[1 1 1] Action with MySession
  (`MySessionSubsystem.CreateSession` (`self.MySessionSubsystem`) 4 (`self.EnableLAN`))
  (`GameplayStatics.OpenLevel` "MultiPlayerMap" true "listen"))

(event `ShowCreateRoom`
  (bind _returnvalue (`GameplayStatics.GetPlayerController` 0))
  (bind _createroom (`self.CreateRoom`))
  (`self.TransitionToState` "NewEnumerator5"
    (:`NewState`
      (`/Engine/EditorBlueprintResources/StandardMacros.IsValid` (`self.CreateRoom`)
        (:`Is Valid`
          _)
        (:`Is Not Valid`
          (bind _returnvalue_2 (`|CreateWidget` "/Game/Blueprints/Widgets/MainMenu/CreateRoom.CreateRoom_C" _returnvalue))
          (set `self.CreateRoom` _returnvalue_2)))
      (`WidgetBlueprintLibrary.SetInputMode_UIOnlyEx` _returnvalue _createroom)
      (`UserWidget.AddToViewport` _createroom 0))))

(event `FindGame(With MySession)`
  ;[1 1 1] Action with MySession
  (`MySessionSubsystem.FindSessions` (`self.MySessionSubsystem`) 0 (`self.EnableLAN`)))

(event `DestroySessionCaller(With MySession)`
  ;[1 1 1] Action with MySession
  (`MySessionSubsystem.DestroySession` (`self.MySessionSubsystem`)))

(event `ShowServerList`
  (bind _returnvalue (`GameplayStatics.GetPlayerController` 0))
  (bind _serverlist (`self.ServerList`))
  (`self.TransitionToState` "NewEnumerator2"
    (:`NewState`
      (`/Engine/EditorBlueprintResources/StandardMacros.IsValid` (`self.ServerList`)
        (:`Is Valid`
          _)
        (:`Is Not Valid`
          (bind _returnvalue_2 (`|CreateWidget` "/Game/Blueprints/Widgets/MainMenu/ServerListMenu.ServerListMenu_C" _returnvalue))
          (set `self.ServerList` _returnvalue_2)))
      (`/Game/Blueprints/Widgets/MainMenu/ServerListMenu.Setup` _serverlist)
      (`WidgetBlueprintLibrary.SetInputMode_UIOnlyEx` _returnvalue _serverlist)
      (`UserWidget.AddToViewport` _serverlist 0)
      (`self.FindGame`))))

(event `SinglePlay`
  (`GameplayStatics.OpenLevel` "MultiPlayerMap"))

(event `ShowLoadingWidget`
  (bind _returnvalue (`GameplayStatics.GetPlayerController` 0))
  (bind _loadingwidget (`self.LoadingWidget`))
  (`self.TransitionToState` "NewEnumerator7"
    (:`NewState`
      (`/Engine/EditorBlueprintResources/StandardMacros.IsValid` (`self.LoadingWidget`)
        (:`Is Valid`
          _)
        (:`Is Not Valid`
          (bind _returnvalue_2 (`|CreateWidget` "/Game/Blueprints/Widgets/MainMenu/LoadingWidget.LoadingWidget_C" _returnvalue))
          (set `self.LoadingWidget` _returnvalue_2)))
      (`UserWidget.AddToViewport` _loadingwidget 0)
      (`WidgetBlueprintLibrary.SetInputMode_UIOnlyEx` _returnvalue _loadingwidget))))

(event `HostGame`
  (params (RoomName :type String) (RoomPassword :type String) (MaxPlayer :type Integer))
  (`CreateSessionCallbackProxyAdvanced.CreateAdvancedSession` (`|MakeArray` (`AdvancedSessionsLibrary.MakeLiteralSessionPropertyString` "RoomName" RoomName) (`AdvancedSessionsLibrary.MakeLiteralSessionPropertyString` "RoomPassword" RoomPassword)) (`GameplayStatics.GetPlayerController` 0) MaxPlayer 0 (`self.EnableLAN`)
    (:`then`
      _)
    (:`OnSuccess`
      _))
  (`GameplayStatics.OpenLevel` "MultiPlayerMap" true "listen"))

(event `FindGame`
  (bind _results (`FindSessionsCallbackProxyAdvanced.FindSessionsAdvanced` (`GameplayStatics.GetPlayerController` 0) 10 (`self.EnableLAN`) "AllServers")
    (:`then`
      (set `self.FindingSessions` true))
    (:`OnSuccess`
      (set `self.FoundSessions` _results)
      (set `self.FindingSessions` false))))

(event `JoinFromServerListEvent`
  (params (Session :type "BlueprintSessionResult Structure"))
  (bind _returnvalue (`GameplayStatics.GetPlayerController` 0))
  (bind _joinroom (`self.JoinRoom`))
  (bind _extrasettings (`AdvancedSessionsLibrary.GetExtraSettings` Session))
  (bind _settingvalue (`AdvancedSessionsLibrary.GetSessionPropertyString` _extrasettings "RoomPassword")
    (:`Found`
      (if (`KismetStringLibrary.EqualEqual_StrStr` _settingvalue)
        (`self.JoinGameSession` Session)
        (else
          (`self.TransitionToState` "NewEnumerator6"
            (:`NewState`
              (`/Engine/EditorBlueprintResources/StandardMacros.IsValid` (`self.JoinRoom`)
                (:`Is Valid`
                  _)
                (:`Is Not Valid`
                  (bind _returnvalue_2 (`|CreateWidget` "/Game/Blueprints/Widgets/MainMenu/JoinRoom.JoinRoom_C" _returnvalue))
                  (bind _output_get (set `self.JoinRoom` _returnvalue_2))))
              (set `/Game/Blueprints/Widgets/MainMenu/JoinRoom.Session` Session _output_get)
              (`WidgetBlueprintLibrary.SetInputMode_UIOnlyEx` _returnvalue _joinroom)
              (`UserWidget.AddToViewport` _joinroom 0))))))))

(event `JoinGame`
  (params (Session :type "BlueprintSessionResult Structure") (Password :type String))
  (bind _extrasettings (`AdvancedSessionsLibrary.GetExtraSettings` Session))
  (bind _settingvalue (`AdvancedSessionsLibrary.GetSessionPropertyString` _extrasettings "RoomPassword")
    (:`Found`
      (if (`KismetStringLibrary.EqualEqual_StrStr` _settingvalue Password)
        (`self.JoinGameSession` Session)))))

(event `JoinGameSession`
  (params (Session :type "BlueprintSessionResult Structure"))
  (`self.ShowLoadingWidget`)
  (`JoinSessionCallbackProxy.JoinSession` (`GameplayStatics.GetPlayerController` 0) Session))

(event `DestroySessionCaller`
  (`DestroySessionCallbackProxy.DestroySession` (`GameplayStatics.GetPlayerController` 0)))

(fn `BeginPlayShowMainMenu`
  (`self.IsCurrentState` "NewEnumerator4"
    (:`True`
      (`self.Setup`)
      (`self.ShowMainMenu`))))

(fn `Setup`
  (set `self.MySessionSubsystem` (subsystem `MySessionSubsystem`)))

(fn `StartPlayingLevel01`
  (`self.Setup`)
  (`self.TransitionToState` "NewEnumerator3"))