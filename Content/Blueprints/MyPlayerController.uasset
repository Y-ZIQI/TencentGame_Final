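; Player controller that manages the in-game HUD, end menu, remaining-time value and leaving the match.
; ClientPostLogin creates the HUD for the local controller and asks MyGameMode to respawn the player.
; Releasing Pause triggers EndGame, which shows the end menu with UI-only input and a visible cursor.
; ExitGame branches on authority, either notifying the game mode or returning to the main menu through MyGameInstance.
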(event `UpdateTime`
  (params (NewTime :type Integer))
  (set `self.RestTime` NewTime))

(event `ClientPostLogin`
  (`self.SetupIngameUI`)
  (bind _asmy_game_mode (cast `/Game/Blueprints/MyGameMode` (`GameplayStatics.GetGameMode`)))
  (`/Game/Blueprints/MyGameMode.RespawnPlayer` _asmy_game_mode self))

(event `InputAction|Pause`
  (params (Key :type "Key Structure"))
  (:`Released`
    (`self.EndGame`)))

(event `EndGame`
  (if (`self.IsLocalPlayerController`)
    (bind _returnvalue (`|CreateWidget` "/Game/Blueprints/Widgets/InGame/EndMenu.EndMenu_C" self))
    (bind _output_get (set `self.EndWidget` _returnvalue))
    (`UserWidget.AddToViewport` _output_get 0)
    (`WidgetBlueprintLibrary.SetInputMode_UIOnlyEx` self _output_get)
    (set `self.bShowMouseCursor` true)))

(event `ExitGame`
  (`/Engine/EditorBlueprintResources/ActorMacros.Switch Has Authority`
    (:`Authority`
      (bind _asmy_game_mode (cast `/Game/Blueprints/MyGameMode` (`GameplayStatics.GetGameMode`)))
      (`/Game/Blueprints/MyGameMode.ClientExitGame` _asmy_game_mode))
    (:`Remote`
      (`self.LocalExitGame`))))

(event `LocalExitGame`
  (bind _asmy_game_instance (cast `/Game/Blueprints/MyGameInstance` (`GameplayStatics.GetGameInstance`)))
  (`/Game/Blueprints/MyGameInstance.ShowMainMenu` _asmy_game_instance))

(fn `SetupIngameUI`
  (if (`self.IsLocalPlayerController`)
    (bind _returnvalue (`|CreateWidget` "/Game/Blueprints/Widgets/InGame/MyHUD.MyHUD_C" self))
    (bind _output_get (set `self.HUDWidget` _returnvalue))
    (`UserWidget.AddToViewport` _output_get 0)))

(fn `UserConstructionScript`)