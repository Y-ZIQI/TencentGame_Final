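; Game mode for a timed multiplayer survival match with Startup, Gaming and GameEnd states, relaying time and results to player controllers.
; Tick drives a per-second countdown that switches phases and periodically spawns player-count-scaled monster waves around the first spawn point.
; Startup logins claim cached PlayerStarts for respawning from a shared team pool.
; Outlasting the timer wins; exhausting respawns or calling LoseGame loses.
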(event `UpdateClientTime`
  (params (NewTime :type Integer))
  (for _array_element (`self.PlayerControllerArray`)
    (`/Engine/EditorBlueprintResources/StandardMacros.IsValid` _array_element
      (:`Is Valid`
        (`/Game/Blueprints/MyPlayerController.UpdateTime` _array_element NewTime)))))

(event `ClientEndGame`
  (params (IsWin :type Boolean))
  (for _array_element (`self.PlayerControllerArray`)
    (`/Engine/EditorBlueprintResources/StandardMacros.IsValid` _array_element
      (:`Is Valid`
        (`/Game/Blueprints/MyPlayerController.LocalEndGame` _array_element IsWin)))))

(event `ClientExitGame`
  (for _array_element (`self.PlayerControllerArray`)
    (`/Engine/EditorBlueprintResources/StandardMacros.IsValid` _array_element
      (:`Is Valid`
        (`/Game/Blueprints/MyPlayerController.LocalExitGame` _array_element)))))

(event `self.ReceiveBeginPlay`
  (`self.ResetTime` (`self.StartupTime`))
  (set `self.GameEnd` false)
  (`self.UpdateClientTime` (`self.RestTimeInt`)))

(event `self.ReceiveTick`
  (params (DeltaSeconds :type "Float (single-precision)"))
  (if (not (`self.GameEnd`))
    (bind _updateclienttime (`self.UpdateTime` DeltaSeconds))
    (if _updateclienttime
      (`self.GameMainProcedure` (`self.RestTimeInt`)))))

(event `RespawnPlayer`
  (params (PlayerControllor :type "/Game/Blueprints/MyPlayerController Object Reference"))
  (bind _returnvalue (`Controller.K2_GetPawn` PlayerControllor))
  (bind _playstartid (`/Game/Blueprints/MyPlayerController.PlayStartId` PlayerControllor))
  (`/Engine/EditorBlueprintResources/StandardMacros.IsValid` _returnvalue
    (:`Is Valid`
      (bind _asthird_person_character (cast `/Game/Blueprints/Actors/ThirdPersonCharacter` _returnvalue)
        (:`then`
          (`/Game/Blueprints/Actors/ThirdPersonCharacter.ThrowAllStaff` _asthird_person_character))
        (:`CastFailed`
          _))
      (`self.K2_DestroyActor` _returnvalue))
    (:`Is Not Valid`
      _))
  (if (>= _playstartid 0)
    (bind _returnvalue_2 (`|SpawnActorFromClass` "/Game/Blueprints/Actors/ThirdPersonCharacter.ThirdPersonCharacter_C" (`self.GetTransform` (`|GetArrayItem` (`self.PlayerStartArray`) _playstartid)) "AdjustIfPossibleButAlwaysSpawn" "OverrideRootScale" null null))
    (`Controller.Possess` PlayerControllor _returnvalue_2)
    (switch `/Game/Blueprints/Level01State` (`self.CurrentState`)
      (:`NewEnumerator1`
        (bind _output_get (set `self.RespawnTime` (- (`self.RespawnTime`) 1)))
        (for _array_element (`self.PlayerControllerArray`)
          (`/Game/Blueprints/MyPlayerController.SetTeamRespawnTimes` _array_element _output_get))
        (if (< _output_get 0)
          (set `self.GameEnd` true)
          (`self.ClientEndGame` false)
          (set `self.CurrentState` "NewEnumerator2"))))))

(event `self.K2_PostLogin`
  (params (NewPlayer :type "PlayerController Object Reference"))
  (switch `/Game/Blueprints/Level01State` (`self.CurrentState`)
    (:`NewEnumerator0`
      (`/Engine/EditorBlueprintResources/ActorMacros.Switch Has Authority`
        (:`Authority`
          (bind _asmy_player_controller (cast `/Game/Blueprints/MyPlayerController` NewPlayer))
          (`KismetArrayLibrary.Array_AddUnique` (`self.PlayerControllerArray`) _asmy_player_controller)
          (bind _startid (`self.getAvailableStart`))
          (if (>= _startid 0)
            (`KismetArrayLibrary.Array_Set` (`self.PlayerStartUsed`) _startid true)
            (set `/Game/Blueprints/MyPlayerController.PlayStartId` _startid _asmy_player_controller))
          (`/Game/Blueprints/MyPlayerController.ClientPostLogin` _asmy_player_controller)
          (`self.RespawnPlayer` _asmy_player_controller))))))

(event `self.K2_OnLogout`
  (params (ExitingController :type "Controller Object Reference"))
  (if (`Controller.IsPlayerController` ExitingController)
    (bind _asmy_player_controller (cast `/Game/Blueprints/MyPlayerController` ExitingController))
    (bind _playstartid (`/Game/Blueprints/MyPlayerController.PlayStartId` _asmy_player_controller))
    (if (>= _playstartid 0)
      (`KismetArrayLibrary.Array_Set` (`self.PlayerStartUsed`) _playstartid)
      (`KismetArrayLibrary.Array_RemoveItem` (`self.PlayerControllerArray`) _asmy_player_controller))))

(event `GameMainProcedure`
  (params (Time :type Integer))
  (bind _playercontrollerarray (`self.PlayerControllerArray`))
  (bind _returnvalue (`KismetArrayLibrary.Array_Length` (`self.PlayerControllerArray`)))
  (`self.UpdateClientTime` Time)
  (if (<= (`self.RestTimeInt`) 0)
    (switch `/Game/Blueprints/Level01State` (`self.CurrentState`)
      (:`NewEnumerator0`
        (`self.ResetTime` (`self.GamingTime`))
        (bind _output_get (set `self.RespawnTime` (+ (`KismetArrayLibrary.Array_Length` _playercontrollerarray) 2)))
        (for _array_element _playercontrollerarray
          (`/Engine/EditorBlueprintResources/StandardMacros.IsValid` _array_element
            (:`Is Valid`
              (`/Game/Blueprints/MyPlayerController.SetTeamRespawnTimes` _array_element _output_get)
              (`self.RespawnPlayer` _array_element))))
        (`KismetSystemLibrary.PrintString` "Game Begins!" true true (struct :`R` 1.0 :`A` 1.0) 5.0)
        (set `self.CurrentState` "NewEnumerator1"))
      (:`NewEnumerator1`
        (set `self.GameEnd` true)
        (`self.ClientEndGame` true)
        (set `self.CurrentState` "NewEnumerator2")))
    (else
      (switch `/Game/Blueprints/Level01State` (`self.CurrentState`)
        (:`NewEnumerator1`
          (bind _output_get_2 (set `self.MonsterSpawnCD` (- (`self.MonsterSpawnCD`) 1)))
          (if (<= _output_get_2 0)
            (set `self.MonsterSpawnCD` (`KismetMathLibrary.RandomIntegerInRange` 3 (- 7 (/ _returnvalue 2))))
            (`self.SpawnMonster` (`KismetMathLibrary.RandomIntegerInRange` (+ _returnvalue 1) (+ _returnvalue 4)))))))))

(event `SpawnMonster`
  (params (Amount :type Integer))
  (bind _output (`|GetArrayItem` (`self.MonsterSpawnArray`)))
  (bind (_randomlocation _returnvalue) (`NavigationSystemV1.K2_GetRandomReachablePointInRadius` (`self.K2_GetActorLocation` _output) 1000.0 null null))
  (for _ (range (+ Amount 1))
    (`/Engine/EditorBlueprintResources/StandardMacros.IsValid` _output
      (:`Is Valid`
        (if _returnvalue
          (`|SpawnActorFromClass` "/Game/Blueprints/Actors/Monster/MonsterCharacter.MonsterCharacter_C" (`KismetMathLibrary.MakeTransform` _randomlocation) "AdjustIfPossibleButAlwaysSpawn" "OverrideRootScale" null null))))))

(event `LoseGame`
  (set `self.GameEnd` true)
  (`self.ClientEndGame` false)
  (set `self.CurrentState` "NewEnumerator2"))

(fn `getAvailableStart`
  (returns (startId :type Integer))
  (for (_array_element _array_index) (`self.PlayerStartUsed`)
    (if (not _array_element)
      (return _array_index)))
  (return -1))

(fn `ResetTime`
  (params (Time :type Integer))
  (set `self.RestTime` (`KismetMathLibrary.Conv_IntToDouble` Time))
  (set `self.RestTimeInt` Time))

(fn `UpdateTime`
  (params (Duration :type "Float (double-precision)"))
  (returns (UpdateClientTime :type Boolean) (RestTimeInt :type Integer))
  (bind _output_get (set `self.RestTime` (- (`self.RestTime`) Duration)))
  (bind _returnvalue (`KismetMathLibrary.FCeil` _output_get))
  (if (!= _returnvalue (`self.RestTimeInt`))
    (bind _output_get_2 (set `self.RestTimeInt` _returnvalue))
    (return true _output_get_2)
    (else
      (return false (`self.RestTimeInt`)))))

(fn `UserConstructionScript`
  (`self.ResetStartArray`
    (:`Output`
      (`self.ResetMonsterSpawn`
        (:`End`
          (`self.ResetNPC`))))))