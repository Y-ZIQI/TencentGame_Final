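; Level 02 game mode that registers joining players and spawns their armed characters.
; On the server, PostLogin stores each controller and calls RespawnPlayer, which destroys any existing pawn, spawns and possesses a PlayerCharacter, then hands it a new Rifle_Ka47.
; The construction script builds the PlayerStart list and parallel used flags, but respawns always use the first start and never check the flags.
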(event `self.K2_PostLogin`
  (params (NewPlayer :type "PlayerController Object Reference"))
  (`/Engine/EditorBlueprintResources/ActorMacros.Switch Has Authority`
    (:`Authority`
      (`KismetArrayLibrary.Array_AddUnique` (`self.PlayerControllerArray`) NewPlayer)
      (`self.RespawnPlayer` NewPlayer))))

(event `RespawnPlayer`
  (params (PlayerController :type "PlayerController Object Reference"))
  (bind _returnvalue (`Controller.K2_GetPawn` PlayerController))
  (`/Engine/EditorBlueprintResources/StandardMacros.IsValid` _returnvalue
    (:`Is Valid`
      (`self.K2_DestroyActor` _returnvalue))
    (:`Is Not Valid`
      _))
  (bind _returnvalue_2 (`|SpawnActorFromClass` "/Game/Blueprints/Actors/PlayerCharacter.PlayerCharacter_C" (`self.GetTransform` (`|GetArrayItem` (`self.PlayerStartArray`))) "AdjustIfPossibleButAlwaysSpawn" "OverrideRootScale" null null))
  (`Controller.Possess` PlayerController _returnvalue_2)
  (bind _returnvalue_3 (`|SpawnActorFromClass` "/Game/Blueprints/Actors/Rifle_Ka47.Rifle_Ka47_C" (`SceneComponent.K2_GetComponentToWorld` (`/Game/Blueprints/Actors/PlayerCharacter.RightClavicleSocket` _returnvalue_2)) "AlwaysSpawn" "OverrideRootScale" null null))
  (`/Game/Blueprints/Actors/PlayerCharacter.PickUpRifle` _returnvalue_2 _returnvalue_3))

(fn `UserConstructionScript`
  (`self.ResetStartArray`))