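; ProtectNPC is a character the player must keep alive, since its death loses the game.
; While Alive, AnyDamage subtracts from HealthPoint, and at zero or below it calls Die and Lose.
; Die clears Alive and ragdolls the mesh with physics-only collision, while Lose calls LoseGame on MyGameMode.
; A helper function sets the character's max walk speed.
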(event `TakeDamage`
  (params (Damage :type "Float (double-precision)"))
  (set `self.HealthPoint` (- (`self.HealthPoint`) Damage)))

(event `self.ReceiveAnyDamage`
  (params (Damage :type "Float (single-precision)") (DamageType :type "DamageType Object Reference") (InstigatedBy :type "Controller Object Reference") (DamageCauser :type "Actor Object Reference"))
  (if (`self.Alive`)
    (`self.TakeDamage` Damage)
    (if (<= (`self.HealthPoint`) 0.0)
      (`self.Die`)
      (`self.Lose`))))

(event `Lose`
  (bind _asmy_game_mode (cast `/Game/Blueprints/MyGameMode` (`GameplayStatics.GetGameMode`)))
  (`/Game/Blueprints/MyGameMode.LoseGame` _asmy_game_mode))

(event `Die`
  (bind _mesh (`self.Mesh`))
  (set `self.Alive` false)
  (`SkeletalMeshComponent.SetAllBodiesSimulatePhysics` _mesh true)
  (`SkeletalMeshComponent.SetAllBodiesPhysicsBlendWeight` _mesh 1.0 false)
  (`PrimitiveComponent.SetCollisionEnabled` _mesh "PhysicsOnly"))

(fn `UpdateWalkSpeed`
  (params (NewSpeed :type "Float (double-precision)"))
  (set `CharacterMovementComponent.MaxWalkSpeed` NewSpeed (`self.CharacterMovement`)))

(fn `UserConstructionScript`)