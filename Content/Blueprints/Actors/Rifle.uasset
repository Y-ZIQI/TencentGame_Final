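; Rifle weapon actor that a ThirdPersonCharacter can detect nearby and that shows a firing effect.
; While the rifle is not Picked, its Sphere overlap adds it to or removes it from the overlapping character's SurroundStaff array.
; Fire and UnFire call ClientFire and ClientUnFire, which only show or hide the GunFire component, with no projectile or damage logic.
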(event `self.Sphere.OnComponentBeginOverlap`
  (params (OverlappedComponent :type "PrimitiveComponent Object Reference") (OtherActor :type "Actor Object Reference") (OtherComp :type "PrimitiveComponent Object Reference") (OtherBodyIndex :type Integer) (bFromSweep :type Boolean) (SweepResult :type "HitResult Structure (by ref)"))
  (if (not (`self.Picked`))
    (bind _asthird_person_character (cast `/Game/Blueprints/Actors/ThirdPersonCharacter` OtherActor))
    (`KismetArrayLibrary.Array_AddUnique` (`/Game/Blueprints/Actors/ThirdPersonCharacter.SurroundStaff` _asthird_person_character) self)))

(event `self.Sphere.OnComponentEndOverlap`
  (params (OverlappedComponent :type "PrimitiveComponent Object Reference") (OtherActor :type "Actor Object Reference") (OtherComp :type "PrimitiveComponent Object Reference") (OtherBodyIndex :type Integer))
  (if (not (`self.Picked`))
    (bind _asthird_person_character (cast `/Game/Blueprints/Actors/ThirdPersonCharacter` OtherActor))
    (`KismetArrayLibrary.Array_RemoveItem` (`/Game/Blueprints/Actors/ThirdPersonCharacter.SurroundStaff` _asthird_person_character) self)))

(event `Fire`
  (`self.ClientFire`))

(event `ClientFire`
  (`SceneComponent.SetVisibility` (`self.GunFire`) true false))

(event `UnFire`
  (`self.ClientUnFire`))

(event `ClientUnFire`
  (`SceneComponent.SetVisibility` (`self.GunFire`) false false))

(fn `UserConstructionScript`)