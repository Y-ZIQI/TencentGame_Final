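; BP_Character is a character Blueprint with health, damage and blood effects, plus helpers to change walk speed and add health capped at the maximum.
; It starts at maximum health, stores its spawn location on BeginPlay and subtracts incoming damage from health.
; Point damage triggers a Bleeding event that attaches a blood emitter to the mesh at the hit location.
; Death is unfinished: the zero-health branch is empty and clearing Alive is unconnected.
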(event `self.ReceiveBeginPlay`
  (set `self.SpawnLocation` (`self.K2_GetActorLocation` self)))

(event `self.ReceiveAnyDamage`
  (params (Damage :type "Float (single-precision)") (DamageType :type "DamageType Object Reference") (InstigatedBy :type "Controller Object Reference") (DamageCauser :type "Actor Object Reference"))
  (bind _output_get (set `self.HealthPoint` (- (`self.HealthPoint`) Damage)))
  (if (<= _output_get 0.0)
    _))

(event `self.ReceivePointDamage`
  (params (Damage :type "Float (single-precision)") (DamageType :type "DamageType Object Reference") (HitLocation :type "Vector Structure") (HitNormal :type "Vector Structure") (HitComponent :type "PrimitiveComponent Object Reference") (BoneName :type Name) (ShotFromDirection :type "Vector Structure") (InstigatedBy :type "Controller Object Reference") (DamageCauser :type "Actor Object Reference") (HitInfo :type "HitResult Structure (by ref)"))
  (`self.Bleeding` (`KismetMathLibrary.MakeTransform` HitLocation)))

(event `Bleeding`
  (params (Location :type "Transform Structure"))
  (`GameplayStatics.SpawnEmitterAttached` "/Game/Blueprints/Particles/P_Blood.P_Blood" (`self.Mesh`) "None" (.location Location) (.rotation Location) (1.0 1.0 1.0) "KeepWorldPosition"))

(fn `UpdateHealthPoint`
  (params (Val :type "Float (double-precision)"))
  (set `self.HealthPoint` (`KismetMathLibrary.FMin` (+ (`self.HealthPoint`) Val) (`self.MaxHealthPoint`))))

(fn `UpdateWalkSpeed`
  (params (NewSpeed :type "Float (double-precision)"))
  (set `CharacterMovementComponent.MaxWalkSpeed` NewSpeed (`self.CharacterMovement`)))

(fn `UserConstructionScript`
  (set `self.HealthPoint` (`self.MaxHealthPoint`)))