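; Enemy Blueprint that carries a spawned AR4 rifle, shoots at the player and reports damage it takes to its EnemyAIController.
; Aim events move the rifle between clavicle and right-hand sockets, with state-guarded wrappers calling Server-prefixed events.
; Attacking starts rifle fire and a looping timer that runs ShootFront until stopped.
; ShootFront line-traces PhysicsBody objects with random spread and debug drawing, damaging only PlayerCharacter hits.
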(event `self.ReceiveBeginPlay`
  (`parent.ReceiveBeginPlay`)
  (`self.PickupRifle` null))

(event `ServerAiming`
  (bind _riflemesh (`self.RifleMesh`))
  (set `self.IsAiming` true)
  (`SceneComponent.K2_AttachToComponent` _riflemesh (`self.RightHandRifleSocket`) "None" "KeepWorld" "KeepWorld" "KeepWorld" true)
  (`KismetSystemLibrary.MoveComponentTo` _riflemesh))

(event `Aiming`
  (if (not (`self.IsAiming`))
    (`self.ServerAiming`)))

(event `ServerNotAiming`
  (bind _riflemesh (`self.RifleMesh`))
  (set `self.IsAiming` false)
  (`SceneComponent.K2_AttachToComponent` _riflemesh (`self.RightClavicleSocket`) "None" "KeepWorld" "KeepWorld" "KeepWorld" true)
  (`KismetSystemLibrary.MoveComponentTo` _riflemesh))

(event `NotAiming`
  (if (`self.IsAiming`)
    (`self.ServerNotAiming`)))

(event `ServerAttacking`
  (set `self.IsAttacking` true)
  (`/Game/Blueprints/Actors/Rifle.Fire` (`self.Rifle`))
  (bind _returnvalue (`KismetSystemLibrary.K2_SetTimerDelegate` (delegate `FireEvent`) 0.1 true))
  (set `self.FireTimer` _returnvalue))

(event `Attacking`
  (if (not (`self.IsAttacking`))
    (`self.ServerAttacking`)))

(event `FireEvent`
  (`self.ShootFront`))

(event `NotAttacking`
  (if (`self.IsAttacking`)
    (`self.ServerNotAttacking`)))

(event `ServerNotAttacking`
  (set `self.IsAttacking` false)
  (`/Game/Blueprints/Actors/Rifle.UnFire` (`self.Rifle`))
  (`KismetSystemLibrary.K2_ClearAndInvalidateTimerHandle` (`self.FireTimer`)))

(event `self.ReceiveAnyDamage`
  (params (Damage :type "Float (single-precision)") (DamageType :type "DamageType Object Reference") (InstigatedBy :type "Controller Object Reference") (DamageCauser :type "Actor Object Reference"))
  (`parent.ReceiveAnyDamage` Damage DamageType InstigatedBy DamageCauser)
  (bind _asenemy_aicontroller (cast `/Game/Blueprints/Actors/Enemy/EnemyAIController` (`self.GetController` self)))
  (`/Game/Blueprints/Actors/Enemy/EnemyAIController.BeingAttacked` _asenemy_aicontroller DamageCauser))

(event `PickupRifle`
  (params (Rifle :type "/Game/Blueprints/Actors/Rifle Object Reference"))
  (bind _returnvalue (`|SpawnActorFromClass` "/Game/Blueprints/Actors/Rifle_AR4.Rifle_AR4_C" (`SceneComponent.K2_GetComponentToWorld` (`self.RightClavicleSocket`)) "AlwaysSpawn" "OverrideRootScale" null null))
  (bind _output_get (set `self.Rifle` _returnvalue))
  (bind _output_get_2 (set `self.RifleMesh` (`/Game/Blueprints/Actors/Rifle.SkeletalMesh` _output_get)))
  (`SceneComponent.K2_AttachToComponent` _output_get_2 (`self.RightClavicleSocket`) "None" "KeepWorld" "KeepWorld" "KeepWorld" true))

(fn `ShootFront`
  (bind _shootarrow (`self.ShootArrow`))
  (bind _returnvalue (`SceneComponent.K2_GetComponentLocation` _shootarrow))
  (bind (_outhit _returnvalue_2) (`KismetSystemLibrary.LineTraceSingleForObjects` :`Start` _returnvalue :`End` (+ _returnvalue (* (+ (* (`KismetMathLibrary.RandomUnitVector`) 0.03) (`SceneComponent.GetForwardVector` _shootarrow)) (`self.FireRange`))) :`ObjectTypes` (`|MakeArray` "ObjectTypeQuery4" :!type "EObjectTypeQuery Enum") :`DrawDebugType` "ForDuration" :`DrawTime` 0.3))
  (if _returnvalue_2
    (bind _asplayer_character (cast `/Game/Blueprints/Actors/PlayerCharacter` (`.HitActor` (`GameplayStatics.BreakHitResult` _outhit))))
    (`GameplayStatics.ApplyDamage` _asplayer_character 1.0 (`self.GetController`) self)))

(fn `UserConstructionScript`
  (`parent.UserConstructionScript`))